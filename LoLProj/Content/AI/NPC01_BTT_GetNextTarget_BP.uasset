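; Behavior tree task for NPC01 that picks the next target point from the controlled character.
; On execute it casts the pawn to BP_TPCharacter and writes the TargetPoints entry at the current Index to a blackboard key.
; It then advances Index, wrapping around the array length so the points cycle in order, and finishes successfully.
; A failed cast stops the graph without calling FinishExecute.
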(event `self.ReceiveExecuteAI`
  (params (OwnerController :type "AIController Object Reference") (ControlledPawn :type "Pawn Object Reference"))
  (bind _asbp_tpcharacter (cast `/Game/BP/BP_TPCharacter` ControlledPawn))
  (bind _targetpoints (`/Game/BP/BP_TPCharacter.TargetPoints` _asbp_tpcharacter))
  (`BTFunctionLibrary.SetBlackboardValueAsObject` (`self.Key`) (`|GetArrayItem` _targetpoints (`self.index`)))
  (set `self.index` (mod (+ (`self.index`) 1) (`KismetArrayLibrary.Array_Length` _targetpoints)))
  (`self.FinishExecute` true))